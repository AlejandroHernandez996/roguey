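; Roguey character Blueprint that sets up the on-screen combat and experience UI at BeginPlay.
; It creates hitsplat and healthbar widgets, assigns itself as their pawn and binds them to damage.
; A target plate widget follows target changes and shows only while the target is valid.
; Each experience drop event spawns a new widget showing the amount gained, with the stat type unused.
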(event Custom|OnTargetPawn_Event
  (params (CurrentTarget :type Roguey%20Pawn%20Object%20Reference))
  (Variables|/Game/Roguey/UI/BP_TargetPlat.BP_TargetPlat_C|SetTargetPawn (stale EventBeginPlay _returnvalue) CurrentTarget)
  (if (Utilities|IsValid CurrentTarget)
    (Widget|SetVisibility (stale EventBeginPlay _returnvalue) "HitTestInvisible")
    (else
      (Widget|SetVisibility (stale EventBeginPlay _returnvalue) "Hidden"))))

(event Custom|Create%20XP_Drop
  (params (ExperienceAmount :type Integer%20%28by%20ref%29) (StatType :type ErogueyStatType%20Enum :default "FLAT_ARMOR"))
  (bind _returnvalue (UserInterface|CreateWidget "/Game/Roguey/UI/BP_Experience_Drop.BP_Experience_Drop_C"))
  (Rendering|Components|TextRender|SetText (Variables|/Game/Roguey/UI/BP_Experience_Drop.BP_Experience_Drop_C|GetExperience_Drop_Text _returnvalue) (Utilities|Text|ToText(Integer) ExperienceAmount))
  (UserInterface|Viewport|AddtoViewport _returnvalue 0))

(event EventTick
  (params (DeltaSeconds :type Float%20%28single-precision%29)))

(event EventBeginPlay
  (bind _self self)
  (bind _returnvalue (UserInterface|CreateWidget "/Game/Roguey/UI/BP_TargetPlat.BP_TargetPlat_C"))
  (Widget|SetVisibility _returnvalue "Hidden")
  (UserInterface|Viewport|AddtoViewport _returnvalue 0)
  (EventDispatchers|AssignOnTargetPawn (delegate Custom|OnTargetPawn_Event))
  (bind _returnvalue_2 (UserInterface|CreateWidget "/Game/Roguey/UI/BP_Hitsplat.BP_Hitsplat_C"))
  (bind _returnvalue_3 (UserInterface|CreateWidget "/Game/Roguey/UI/BP_Healthbar.BP_Healthbar_C"))
  (bind _output_get (Variables|Default|SetHitsplat _returnvalue_2))
  (bind _output_get_2 (Variables|Default|SetHealthbar _returnvalue_3))
  (UserInterface|Viewport|AddtoViewport _output_get_2 0)
  (UserInterface|Viewport|AddtoViewport _output_get 0)
  (Variables|/Game/Roguey/UI/BP_Hitsplat.BP_Hitsplat_C|SetPawn (Variables|Default|GetHitsplat) _self)
  (Default|BindonDamageHitsplat (Variables|Default|GetHitsplat))
  (Variables|/Game/Roguey/UI/BP_Healthbar.BP_Healthbar_C|SetPawn (Variables|Default|GetHealthbar) _self)
  (Default|BindonDamageHealthbar (Variables|Default|GetHealthbar))
  (EventDispatchers|BindEventtoOnExperienceDrop (delegate Custom|Create%20XP_Drop)))

(fn ConstructionScript)