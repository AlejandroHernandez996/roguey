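; Roguey pawn Blueprint that shows on-screen damage feedback.
; On BeginPlay it binds to its damage event dispatcher.
; Each damage event creates a new hitsplat widget with the damage amount as text and a new healthbar widget, passes both the owning pawn, and adds them to the viewport.
; Nothing here reuses or removes those widgets.
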(event Custom|OnDamageEvent_Event
  (params (DamageAmount :type Integer%20%28by%20ref%29) (OwningPawn :type Roguey%20Pawn%20Object%20Reference))
  (bind _returnvalue (UserInterface|CreateWidget "/Game/Roguey/UI/BP_Hitsplat.BP_Hitsplat_C"))
  (Rendering|Components|TextRender|SetText (Variables|/Game/Roguey/UI/BP_Hitsplat.BP_Hitsplat_C|GetDamageAmount _returnvalue) (Utilities|Text|ToText(Integer) DamageAmount))
  (Variables|/Game/Roguey/UI/BP_Hitsplat.BP_Hitsplat_C|SetPawn _returnvalue OwningPawn)
  (UserInterface|Viewport|AddtoViewport _returnvalue 0)
  (bind _returnvalue_2 (UserInterface|CreateWidget "/Game/Roguey/UI/BP_Healthbar.BP_Healthbar_C"))
  (Variables|/Game/Roguey/UI/BP_Healthbar.BP_Healthbar_C|SetPawn _returnvalue_2 OwningPawn)
  (UserInterface|Viewport|AddtoViewport _returnvalue_2 0))

(event EventBeginPlay
  (EventDispatchers|AssignOnDamageEvent (delegate Custom|OnDamageEvent_Event)))

(event Collision|EventActorBeginOverlap
  (params (OtherActor :type Actor%20Object%20Reference)))

(event EventTick
  (params (DeltaSeconds :type Float%20%28single-precision%29)))

(fn ConstructionScript)