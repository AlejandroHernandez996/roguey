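; BP_ItemActor is an item actor in Roguey that displays on-screen UI for the item it carries.
; On BeginPlay it adds a collection log widget with the item's name and icon, plus a name indicator widget linked back to itself.
; Every Tick it shows the indicator and refreshes its text, appending the quantity for stackable items.
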(event EventBeginPlay
  (bind _self self)
  (bind _returnvalue (UserInterface|CreateWidget "/Game/Roguey/UI/UI_Animatin/BP_Collection_Log.BP_Collection_Log_C"))
  (Rendering|Components|TextRender|SetText (Variables|/Game/Roguey/UI/UI_Animatin/BP_Collection_Log.BP_Collection_Log_C|GetItem_Name _returnvalue) (Utilities|Text|ToText(String) (.itemname (Variables|Default|GetItem _self))))
  (Appearance|SetBrushfromTexture (Variables|/Game/Roguey/UI/UI_Animatin/BP_Collection_Log.BP_Collection_Log_C|GetIcon _returnvalue) (.itemicon (Variables|Default|GetItem _self)) false)
  (UserInterface|Viewport|AddtoViewport _returnvalue 0)
  (bind _returnvalue_2 (UserInterface|CreateWidget "/Game/Roguey/UI/BP_Item_Name_Idicator.BP_Item_Name_Idicator_C"))
  (UserInterface|Viewport|AddtoViewport _returnvalue_2 0)
  (Variables|/Game/Roguey/UI/BP_Item_Name_Idicator.BP_Item_Name_Idicator_C|SetItem _returnvalue_2 _self)
  (if (.bisstackable (Variables|Default|GetItem _self))
    (Rendering|Components|TextRender|SetText (Variables|/Game/Roguey/UI/BP_Item_Name_Idicator.BP_Item_Name_Idicator_C|GetItemName _returnvalue_2) (Utilities|Text|FormatText "{name} ({qty})" (.itemname (Variables|Default|GetItem _self)) (.quantity (Variables|Default|GetItem _self))))
    (else
      (Rendering|Components|TextRender|SetText (Variables|/Game/Roguey/UI/BP_Item_Name_Idicator.BP_Item_Name_Idicator_C|GetItemName _returnvalue_2) (Utilities|Text|ToText(String) (.itemname (Variables|Default|GetItem _self)))))))

(event Collision|EventActorBeginOverlap
  (params (OtherActor :type Actor%20Object%20Reference)))

(event EventTick
  (params (DeltaSeconds :type Float%20%28single-precision%29))
  (bind _self self)
  (bind _item (Variables|Default|GetItem _self))
  (Default|ShowText (stale EventBeginPlay _returnvalue_2))
  (if (.bisstackable _item)
    (Rendering|Components|TextRender|SetText (Variables|/Game/Roguey/UI/BP_Item_Name_Idicator.BP_Item_Name_Idicator_C|GetItemName (stale EventBeginPlay _returnvalue_2)) (Utilities|Text|FormatText "{name} ({qty})" (.itemname _item) (.quantity _item)))
    (else
      (Rendering|Components|TextRender|SetText (Variables|/Game/Roguey/UI/BP_Item_Name_Idicator.BP_Item_Name_Idicator_C|GetItemName (stale EventBeginPlay _returnvalue_2)) (Utilities|Text|ToText(String) (.itemname _item))))))

(fn ConstructionScript)