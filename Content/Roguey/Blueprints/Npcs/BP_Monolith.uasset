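; BP_Monolith is an NPC Blueprint in Roguey that sets up its own on-screen damage feedback.
; On BeginPlay it creates hitsplat and healthbar widgets, adds both to the viewport and passes itself to each as the Pawn.
; Each widget's bind function is then called to hook it to damage, with no other logic defined in this graph.
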(event EventBeginPlay
  (bind _self self)
  (bind _returnvalue (UserInterface|CreateWidget "/Game/Roguey/UI/BP_Hitsplat.BP_Hitsplat_C"))
  (bind _returnvalue_2 (UserInterface|CreateWidget "/Game/Roguey/UI/BP_Healthbar.BP_Healthbar_C"))
  (bind _output_get (Variables|Default|SetHitsplat _returnvalue))
  (bind _output_get_2 (Variables|Default|SetHealthbar _returnvalue_2))
  (UserInterface|Viewport|AddtoViewport _output_get_2 0)
  (UserInterface|Viewport|AddtoViewport _output_get 0)
  (Variables|/Game/Roguey/UI/BP_Hitsplat.BP_Hitsplat_C|SetPawn (Variables|Default|GetHitsplat) _self)
  (Default|BindonDamageHitsplat (Variables|Default|GetHitsplat))
  (Variables|/Game/Roguey/UI/BP_Healthbar.BP_Healthbar_C|SetPawn (Variables|Default|GetHealthbar) _self)
  (Default|BindonDamageHealthbar (Variables|Default|GetHealthbar)))

(fn ConstructionScript)